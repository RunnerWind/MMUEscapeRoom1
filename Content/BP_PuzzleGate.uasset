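; BP_PuzzleGate is a gate that opens once enough items have been collected to finish a challenge.
; CollectItem counts items and, once the maximum is reached, fires a single time to call OpenDoor and Completed.
; OpenDoor swings the Door's yaw open with a timeline.
; Completed, also guarded by DoOnce, increments the player character's CompletedChallenge count and moves it to a hardcoded location.
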(event `self.ReceiveBeginPlay`)

(event `Open Door`
  (bind (_direction _door_rotation) (`Timeline|Open Door Anim`)
    (:`Update`
      (`SceneComponent.K2_SetRelativeRotation` (`self.Door`) (`KismetMathLibrary.MakeRotator` 0.0 0.0 (`KismetMathLibrary.Lerp` 0.0 120.0 _door_rotation)) false false))))

(event `Collect Item`
  (`/Engine/EditorBlueprintResources/StandardMacros.IncrementInt` (`self.currentItemCollected`)
    (:`  `
      (if (>= (`self.currentItemCollected`) (`self.maxItemCollectable`))
        (`/Engine/EditorBlueprintResources/StandardMacros.DoOnce` false
          (:`Completed`
            (`self.Open Door`)
            (`self.Completed`)))))))

(event `Completed`
  (`/Engine/EditorBlueprintResources/StandardMacros.DoOnce` false
    (:`Completed`
      (bind _asbp_third_person_character (cast `/Game/ThirdPerson/Blueprints/BP_ThirdPersonCharacter` (`GameplayStatics.GetPlayerCharacter` 0)))
      (set `/Game/ThirdPerson/Blueprints/BP_ThirdPersonCharacter.Completed Challenge` (+ (`/Game/ThirdPerson/Blueprints/BP_ThirdPersonCharacter.Completed Challenge` _asbp_third_person_character) 1) _asbp_third_person_character)
      (`self.K2_SetActorLocation` _asbp_third_person_character (500.0 500.0 10.0) false false))))

(fn `UserConstructionScript`)