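; The_endPod is an actor that acts as an on/off toggle triggered by the player character.
; Each time a BP_ThirdPersonCharacter begins overlapping its BoxCollision, the IsOn flag flips.
; Tick reapplies the matching on or off material to the Cube every frame, rather than only when the state changes.
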(event `self.ReceiveTick`
  (params (DeltaSeconds :type "Float (single-precision)"))
  (bind _cube (`self.Cube`))
  (if (`self.isOn?`)
    (`PrimitiveComponent.SetMaterial` _cube 0 "/Game/Blueprint/isOn.isOn")
    (else
      (`PrimitiveComponent.SetMaterial` _cube 0 "/Game/Blueprint/isOff.isOff"))))

(event `self. Box collision.OnComponentBeginOverlap`
  (params (OverlappedComponent :type "PrimitiveComponent Object Reference") (OtherActor :type "Actor Object Reference") (OtherComp :type "PrimitiveComponent Object Reference") (OtherBodyIndex :type Integer) (bFromSweep :type Boolean) (SweepResult :type "HitResult Structure (by ref)"))
  (if (== (`GameplayStatics.GetObjectClass` OtherActor) "/Game/ThirdPerson/Blueprints/BP_ThirdPersonCharacter.BP_ThirdPersonCharacter_C")
    (if (`self.isOn?`)
      (set `self.isOn?` false)
      (else
        (set `self.isOn?` true)))))

(fn `UserConstructionScript`)